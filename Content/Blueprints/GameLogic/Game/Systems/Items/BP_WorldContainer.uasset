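; BP_WorldContainer is a world container actor that fills its inventory with random items on BeginPlay.
; A loop picks random numbered rows from DT_ItemTableTest, gives each item a random 2D position in the bag, and sends it to BPCInventoryBase through ServerAddItem.
; GetInventoryReference exposes that inventory component to other code.
; The fill has no authority check of its own.
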(event EventBeginPlay
  (|CallParentFunction)
  (for _index (range 0 5)
    (bind _returnvalue (Utilities|GetDataTableRow "/Game/Blueprints/DataTables/DT_ItemTableTest.DT_ItemTableTest" (Utilities|String|StringToName (Utilities|String|ToString(Integer) (Math|Random|RandomIntegerinRange 1 7))))
      (:then
        (bind _structout (Utilities|Struct|SetmembersinS_ItemInfo _returnvalue (Math|Vector2D|MakeVector2D (Math|Random|RandomFloatinRange 5.0 3e+02) (Math|Random|RandomFloatinRange 1e+02 2.5e+02))))
        (Default|ServerAddItem (Variables|Default|GetBPC_InventoryBase) _structout)))))

(event Collision|EventActorBeginOverlap
  (params (OtherActor :type Actor%20Object%20Reference))
  (|CallParentFunction OtherActor) ; This node is disabled and will not be called.\nDrag off pins to build functionality.
)

(event EventTick
  (params (DeltaSeconds :type Float%20%28single-precision%29))
  (|CallParentFunction DeltaSeconds) ; This node is disabled and will not be called.\nDrag off pins to build functionality.
)

(fn ConstructionScript
  (|CallParentFunction))

(fn GetInventoryReference
  (return (Variables|Default|GetBPC_InventoryBase)))